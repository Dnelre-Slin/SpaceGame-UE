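; SquareBlockBP is an actor that hosts a two-part interactive door through its InteractiveDoorComponentBP.
; Its construction script adds two manually attached static mesh components and an actor sequence component, then passes them to the component's SetupDoor.
; The event graph holds only disabled stubs, and an unconnected earlier version that placed and attached two BasicDoor meshes directly remains in the construction script.
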(fn `UserConstructionScript`
  (bind _returnvalue (`AddComponent|NODE_AddStaticMeshComponent-2` :`bManualAttachment` true))
  (bind _returnvalue_2 (`AddComponent|NODE_AddStaticMeshComponent-3` :`bManualAttachment` true))
  (bind _returnvalue_3 (`AddComponent|NODE_AddActorSequenceComponent-0`))
  (`/Game/Blueprints/InteractiveDoorComponentBP.SetupDoor` (`self.InteractiveDoorComponentBP`) _returnvalue _returnvalue_2 _returnvalue_3))