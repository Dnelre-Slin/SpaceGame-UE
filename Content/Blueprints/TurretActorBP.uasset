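; TurretActorBP is a turret-named actor Blueprint that has no working behavior; it reads as a scratch asset for quaternion and rotation nodes.
; Its events and construction script are empty, and the event graph holds only unreached calls and unused conversion nodes.
; Awesomeness converts a vector scaled by the sum of two inputs to a quaternion, while Badassness is empty and Magical and NewMacro_0 contain only unused nodes.
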(fn `Awesomeness`
  (params (A :type "Float (double-precision)" :default 1.0) (B :type "Float (double-precision)") (V :type "Vector Structure" :default (3.0 0.0 0.0)))
  (returns (Res :type "Quat Structure"))
  (return (`KismetMathLibrary.Conv_VectorToQuaternion` (* V (+ A B)))))

(fn `Badassness`)

(fn `UserConstructionScript`)