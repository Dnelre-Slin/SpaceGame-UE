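; Turret actor that aims at a target and spawns bullets.
; The construction script chains the top to the stand and the stand to the base via mesh sockets.
; Tick passes the stand and top components to AimAtTarget, which is defined outside these graphs.
; The Fire event spawns a BulletBP at the turret top's world transform, with its trigger also outside this Blueprint.
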(event `self.ReceiveBeginPlay`)

(event `self.ReceiveTick`
  (params (DeltaSeconds :type "Float (single-precision)"))
  (`self.AimAtTarget` DeltaSeconds (`self.TurretStand`) (`self.TurretTop`)))

(event `Fire`
  (`|SpawnActorFromClass` "/Game/Blueprints/BulletBP.BulletBP_C" (`SceneComponent.K2_GetComponentToWorld` (`self.TurretTop`)) "Undefined" "OverrideRootScale" null null))

(fn `UserConstructionScript`
  (`SceneComponent.K2_AttachToComponent` (`self.TurretTop`) (`self.TurretStand`) "TurretTopSocket" "KeepRelative" "KeepRelative" "KeepRelative" true)
  (`SceneComponent.K2_AttachToComponent` (`self.TurretStand`) (`self.TurretBase`) "TurretStandSocket" "KeepRelative" "KeepRelative" "KeepRelative" true))