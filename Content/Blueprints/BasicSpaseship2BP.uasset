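; Player-possessable spaceship Blueprint with interactables for taking control of the ship and opening its door.
; The construction script links each interactable to its reactable and gives the door reactable its opening sequence.
; Possession sets a flag so the next Tick, if an InputComponent exists, passes it to every component implementing InputBindingComponentInterface for binding setup.
; The flag clears after that single attempt, and debug strings trace possession changes.
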(event `self.ReceiveTick`
  (params (DeltaSeconds :type "Float (single-precision)"))
  (bind _returnvalue (`self.GetComponentByClass` "/Script/Engine.InputComponent"))
  (if (`self.RecentlyPossessed`)
    (`KismetSystemLibrary.PrintString` "Possessed, but not yet created")
    (set `self.RecentlyPossessed` false)
    (if (`KismetSystemLibrary.IsValid` _returnvalue)
      (for _array_element (`self.GetComponentsByInterface` "/Script/SpaceGame.InputBindingComponentInterface")
        (message `InputBindingComponentInterface.SetupInputBindings` _array_element _returnvalue)))))

(event `self.ReceivePossessed`
  (params (NewController :type "Controller Object Reference"))
  (`KismetSystemLibrary.PrintString` "SpaceShip Possessed")
  (set `self.RecentlyPossessed` true))

(event `self.ReceiveUnpossessed`
  (params (OldController :type "Controller Object Reference"))
  (`KismetSystemLibrary.PrintString` "Spaceship unpossessed"))

(fn `UserConstructionScript`
  (bind _dooropenreactable (`self.DoorOpenReactable`))
  (`Single2SInteractableComponent.SetReactable` (`self.PossessShipInteractable`) (`self.PossessionReactable`))
  (`Single2SInteractableComponent.SetReactable` (`self.OpenDoorInteractable`) _dooropenreactable)
  (`Sequence2SManuReactableComponent.SetSequence` _dooropenreactable (`self.OpenDoorSequence`)))